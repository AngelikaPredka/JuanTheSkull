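; BP_Mushroom is an edible mushroom actor that either kills or feeds the first-person player.
; It caches the player character on BeginPlay and shows an "Eat[E]" prompt on that character when a look-at hit is reported.
; When used through the interaction interface, a toxic mushroom hides, triggers PlayerDeath after a delay, then reappears.
; A safe one calls MushroomEaten and destroys itself.
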(event `self.ReceiveBeginPlay`
  (`self.EnableInput` (`GameplayStatics.GetPlayerController` 0))
  (bind _asbp_first_person_character (cast `/Game/FirstPerson/Blueprints/BP_FirstPersonCharacter` (`GameplayStatics.GetPlayerCharacter` 0)))
  (set `self.As BP First Person Character` _asbp_first_person_character))

(event `/Game/FirstPerson/Blueprints/BPI_Use.UseInterface`
  (params (NewParam :type "Actor Object Reference"))
  (bind _as_bp_first_person_character (`self.As BP First Person Character`))
  (if (== NewParam self)
    (if (`self.isToxic`)
      (`SceneComponent.SetVisibility` (`self.StaticMesh`) false false)
      (`KismetSystemLibrary.Delay` 3.0)
      (`/Game/FirstPerson/Blueprints/BP_FirstPersonCharacter.PlayerDeath` _as_bp_first_person_character)
      (`KismetSystemLibrary.Delay` 2.0)
      (`SceneComponent.SetVisibility` (`self.StaticMesh`) true false)
      (else
        (`/Game/FirstPerson/Blueprints/BP_FirstPersonCharacter.MushroomEaten` _as_bp_first_person_character)
        (`self.K2_DestroyActor`)))))

(event `/Game/FirstPerson/Blueprints/BPI_Enemy.TransferHitLocation`
  (params (Hit :type Boolean) (NewParam :type "Actor Object Reference"))
  ;[1 1 1] Tylko tu widget spawnawnay jak sie patrzmyy na to
  (if Hit
    (message `/Game/FirstPerson/Blueprints/BPI_Text.SetText` (`self.As BP First Person Character`) "Eat[E]")))

(fn `UserConstructionScript`)