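; BP_Lily is a colored lily platform that sinks when the player character steps into its capsule trigger and rises back when they leave.
; A timeline lerps the cylinder's world Z between its BeginPlay location and that height minus an Offset, played from start on overlap and reversed from the end on exit.
; The Color variable is written to custom primitive data in construction and at BeginPlay, allowing per-instance tint.
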(event `self.ReceiveBeginPlay`
  (bind (_color_r _color_g _color_b) (break `LinearColor` (`self.Color`)))
  (`PrimitiveComponent.SetCustomPrimitiveDataVector4` (`self.Cylinder`) 0 (`KismetMathLibrary.MakeVector4` _color_r _color_g _color_b 1.0))
  (set `self.InitialLocation` (`SceneComponent.K2_GetComponentLocation` (`self.Cylinder`))))

(event `self.Capsule.OnComponentBeginOverlap`
  (params (OverlappedComponent :type "PrimitiveComponent Object Reference") (OtherActor :type "Actor Object Reference") (OtherComp :type "PrimitiveComponent Object Reference") (OtherBodyIndex :type Integer) (bFromSweep :type Boolean) (SweepResult :type "HitResult Structure (by ref)"))
  (bind (_initiallocation_x _initiallocation_y _initiallocation_z) (`KismetMathLibrary.BreakVector` (`self.InitialLocation`)))
  (if (== (`GameplayStatics.GetPlayerCharacter` 0) OtherActor)
    (bind (_direction _newtrack_0) (`Timeline|Timeline` :!via `PlayFromStart` :!label _label)
      (:`Update`
        (`SceneComponent.K2_SetWorldLocation` (`self.Cylinder`) (`KismetMathLibrary.MakeVector` _initiallocation_x _initiallocation_y (`KismetMathLibrary.Lerp` _initiallocation_z (- _initiallocation_z (`self.Offset`)) _newtrack_0)) false false)))))

(event `self.Capsule.OnComponentEndOverlap`
  (params (OverlappedComponent :type "PrimitiveComponent Object Reference") (OtherActor :type "Actor Object Reference") (OtherComp :type "PrimitiveComponent Object Reference") (OtherBodyIndex :type Integer))
  (if (== OtherActor (`GameplayStatics.GetPlayerCharacter` 0))
    (goto _label :!via `ReverseFromEnd`)))

(fn `UserConstructionScript`
  (bind (_color_r _color_g _color_b) (break `LinearColor` (`self.Color`)))
  (`PrimitiveComponent.SetCustomPrimitiveDataVector4` (`self.Cylinder`) 0 (`KismetMathLibrary.MakeVector4` _color_r _color_g _color_b 1.0)))