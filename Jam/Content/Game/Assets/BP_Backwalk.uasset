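; BP_Backwalk is a view-dependent trick actor whose cube moves away or returns depending on which way the player looks.
; Overlapping its box starts a fast looping timer that compares the first-person camera's forward vector with an arrow component's via dot product.
; Facing along the arrow sends the cube to a fixed elevated world position; otherwise it returns to its BeginPlay transform.
; Ending the overlap clears the timer.
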(event `self.ReceiveBeginPlay`
  (bind _asbp_first_person_character (cast `/Game/FirstPerson/Blueprints/BP_FirstPersonCharacter` (`GameplayStatics.GetPlayerCharacter` 0)))
  (set `self.As BP First Person Character` _asbp_first_person_character)
  (set `self.NewVar` (`SceneComponent.K2_GetComponentToWorld` (`self.Cube`))))

(event `Timer`
  (bind _cube (`self.Cube`))
  (bind (_newvar_location _newvar_rotation _newvar_scale) (`KismetMathLibrary.BreakTransform` (`self.NewVar`)))
  (if (> (`KismetMathLibrary.Dot_VectorVector` (`SceneComponent.GetForwardVector` (`/Game/FirstPerson/Blueprints/BP_FirstPersonCharacter.FirstPersonCamera` (`self.As BP First Person Character`))) (`SceneComponent.GetForwardVector` (`self.Arrow`))) 0.5)
    (`SceneComponent.K2_SetWorldTransform` _cube (`KismetMathLibrary.MakeTransform` (- (1.0 1.0 1.0) (0.0 0.0 -1000.0)) _newvar_rotation _newvar_scale) false false)
    (else
      (`SceneComponent.K2_SetWorldTransform` _cube (`KismetMathLibrary.MakeTransform` _newvar_location _newvar_rotation _newvar_scale) false false))))

(event `self.Box.OnComponentBeginOverlap`
  (params (OverlappedComponent :type "PrimitiveComponent Object Reference") (OtherActor :type "Actor Object Reference") (OtherComp :type "PrimitiveComponent Object Reference") (OtherBodyIndex :type Integer) (bFromSweep :type Boolean) (SweepResult :type "HitResult Structure (by ref)"))
  (bind _returnvalue (`KismetSystemLibrary.K2_SetTimerDelegate` (delegate `Timer`) 0.1 true))
  (set `self.NewVar_0` _returnvalue))

(event `self.Box.OnComponentEndOverlap`
  (params (OverlappedComponent :type "PrimitiveComponent Object Reference") (OtherActor :type "Actor Object Reference") (OtherComp :type "PrimitiveComponent Object Reference") (OtherBodyIndex :type Integer))
  (`KismetSystemLibrary.K2_ClearAndInvalidateTimerHandle` (`self.NewVar_0`)))

(fn `UserConstructionScript`)