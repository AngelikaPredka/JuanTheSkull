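; BP_Log is an interactable log that flips over once when the player uses it while strong.
; It caches the first-person character on BeginPlay, and UseInterface checks that the event targets this log and that PlayerIsStrong is set.
; A DoOnce then plays a timeline that lerps the static mesh's relative rotation through a near half-turn along the shortest path.
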(event `self.ReceiveBeginPlay`
  (bind _asbp_first_person_character (cast `/Game/FirstPerson/Blueprints/BP_FirstPersonCharacter` (`GameplayStatics.GetPlayerCharacter` 0)))
  (set `self.As BP First Person Character` _asbp_first_person_character))

(event `/Game/FirstPerson/Blueprints/BPI_Use.UseInterface`
  (params (NewParam :type "Actor Object Reference"))
  (if (== NewParam self)
    (if (`/Game/FirstPerson/Blueprints/BP_FirstPersonCharacter.PlayerIsStrong` (`self.As BP First Person Character`))
      (`/Engine/EditorBlueprintResources/StandardMacros.DoOnce` false
        (:`Completed`
          (bind (_direction _newtrack_0) (`Timeline|Timeline` :!via `PlayFromStart`)
            (:`Update`
              (`SceneComponent.K2_SetRelativeRotation` (`self.StaticMesh`) (`KismetMathLibrary.RLerp` (struct) (struct :`Roll` -179.0) _newtrack_0 true) false false))))))))

(fn `UserConstructionScript`)